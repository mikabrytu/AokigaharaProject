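; BP_Player is the player character, handling basic movement, looking and sprinting.
; Axis inputs move it along the actor's forward and right vectors and drive controller yaw and pitch, with the vertical look input inverted.
; BeginPlay sets the walk speed, and holding Sprint swaps the Character Movement max walk speed to the run speed until release.
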(event EventBeginPlay
  (Variables|/Script/Engine.CharacterMovementComponent|SetMaxWalkSpeed (Variables|Character|GetCharacterMovement) (Variables|Default|GetWalkSpeed)))

(event Collision|EventActorBeginOverlap
  (params (OtherActor :type Actor%20Object%20Reference)))

(event EventTick
  (params (DeltaSeconds :type Float%20%28single-precision%29)))

(event Input|ActionEvents|InputActionSprint
  (params (Key :type Key%20Structure))
  (bind _charactermovement (Variables|Character|GetCharacterMovement))
  ;[1 1 1] Sprint System
  (:Pressed
    (Variables|/Script/Engine.CharacterMovementComponent|SetMaxWalkSpeed _charactermovement (Variables|Default|GetRunSpeed)))
  (:Released
    (Variables|/Script/Engine.CharacterMovementComponent|SetMaxWalkSpeed _charactermovement (Variables|Default|GetWalkSpeed))))

(event Input|AxisEvents|InputAxisMoveForward
  (params (AxisValue :type Float%20%28single-precision%29))
  ;[1 1 1] Basic Movement - Forward and Side
  (Pawn|Input|AddMovementInput (Transformation|GetActorForwardVector) AxisValue false))

(event Input|AxisEvents|InputAxisMoveRight
  (params (AxisValue :type Float%20%28single-precision%29))
  ;[1 1 1] Basic Movement - Forward and Side
  (Pawn|Input|AddMovementInput (Transformation|GetActorRightVector) AxisValue false))

(event Input|AxisEvents|InputAxisLookHorizontal
  (params (AxisValue :type Float%20%28single-precision%29))
  ;[1 1 1] Looking Around Handler
  (Pawn|Input|AddControllerYawInput AxisValue))

(event Input|AxisEvents|InputAxisLookVertical
  (params (AxisValue :type Float%20%28single-precision%29))
  ;[1 1 1] Looking Around Handler
  (Pawn|Input|AddControllerPitchInput (* AxisValue -1.0)))

(fn ConstructionScript)